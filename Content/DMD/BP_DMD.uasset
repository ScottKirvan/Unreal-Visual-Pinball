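; BP_DMD is an actor that shows live DMD (dot-matrix display) output from an emulated ROM on a mesh.
; It starts the Vp backend with RomName on BeginPlay and stops it on EndPlay.
; Each tick it reads the DMD array, writes each value into the red channel of a vertex color, and applies the array as the static mesh's vertex color override, one vertex per element.
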(event EventBeginPlay
  (Class|VPmame|VpStart (Variables|Default|GetRom%20Name)))

(event EventTick
  (params (DeltaSeconds :type Float%20%28single-precision%29))
  (bind _vertexcolors (Variables|Default|GetVertexColors))
  (bind _dots (Class|VPmame|VpGetDMD))
  (for (_array_element _array_index) _dots
    (Utilities|Array|SetArrayElem _vertexcolors _array_index (Math|Color|MakeColor 0 0 _array_element) true))
  (Class|VPmame|SetVertexColorOverride (Variables|Debug|GetStaticMeshComponent) _vertexcolors))

(event EventEndPlay
  (params (EndPlayReason :type EEndPlayReason%20Enum :default "Destroyed"))
  (Class|VPmame|VpStop))

(fn ConstructionScript)